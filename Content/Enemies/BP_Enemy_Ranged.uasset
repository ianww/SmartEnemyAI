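; BP_Enemy_Ranged is a ranged enemy that arms itself with a rifle when play begins.
; EquipWeapon spawns BP_Weapon_Rifle, stores it as WeaponActor and attaches it to the mesh's right-hand rifle socket.
; The attach result sets IsWieldingWeapon, then CallOnWeaponEquipped fires.
; The Attack event is empty, and the construction script only runs the parent's.
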(event EventBeginPlay
  (CallFunction|EquipWeapon))

(event EventEquipWeapon
  (bind _returnvalue (Game|SpawnActorfromClass "/Game/Weapons/BP_Weapon_Rifle.BP_Weapon_Rifle_C" (Math|Transform|MakeTransform "0, 0, 0") "Undefined" "MultiplyWithRoot" 0 0))
  (bind _output_get (Variables|Default|SetWeaponActor _returnvalue))
  (bind _returnvalue_2 (Transformation|AttachComponentToComponent _output_get (Variables|Character|GetMesh) "hand_r_rifle_socket" "KeepRelative" "KeepRelative" "KeepRelative" true))
  (Variables|Default|SetIsWieldingWeapon _returnvalue_2)
  (Default|CallOnWeaponEquipped))

(event EventAttack)

(fn ConstructionScript
  (|CallParentFunction))