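; Melee enemy Blueprint that handles sword attacks and equipping or unequipping the weapon through montages.
; Attack plays a slash and fires OnAttackEnd on completion or interruption.
; Equip and unequip use montage notifies to spawn the sword at the hand socket or destroy it, updating IsWieldingWeapon.
; Their equipped and unequipped dispatchers fire only when the montage completes.
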(event EventEquipWeapon
  (bind _notifyname (Animation|Montage|PlayMontage (Variables|Character|GetMesh) "/Game/Animations/Melee/Montage_UnsheathSword.Montage_UnsheathSword")
    (:OnCompleted
      (Default|CallOnWeaponEquipped))
    (:OnNotifyBegin
      (switch name _notifyname
        (:HoldSword
          (Game|SpawnActorfromClass "/Game/Weapons/BP_Weapon_Sword.BP_Weapon_Sword_C" (Transformation|GetActorTransform) "Undefined" "MultiplyWithRoot" 0 0)
          ;[1 0.7867 0.02475 1 9] BP_Weapon_Sword is a child of BP_Weapon_Base, so it can be assigned to the same variable
          (bind _output_get (Variables|Default|SetWeaponActor 0))
          (Transformation|AttachComponentToComponent _output_get (Variables|Character|GetMesh) "hand_r_sword_socket" "SnapToTarget" "SnapToTarget" "SnapToTarget" true)
          (Variables|Default|SetIsWieldingWeapon true))))))

(event EventUnequipWeapon
  (bind _notifyname (Animation|Montage|PlayMontage (Variables|Character|GetMesh) "/Game/Animations/Melee/Montage_SheathSword.Montage_SheathSword")
    (:OnCompleted
      (Default|CallOnWeaponUnequipped))
    (:OnNotifyBegin
      (switch name _notifyname
        (:DropSword
          (Actor|DestroyActor (Variables|Default|GetWeaponActor))
          (Variables|Default|SetIsWieldingWeapon false))))))

(event EventAttack
  (Animation|Montage|PlayMontage (Variables|Character|GetMesh) "/Game/Animations/Melee/Montage_SwordSlash.Montage_SwordSlash"
    (:OnCompleted
      _)
    (:OnInterrupted
      _))
  (Default|CallOnAttackEnd) ; EventDispatcher
)

(fn ConstructionScript
  (|CallParentFunction))